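; BP_CharacterController is a controller that toggles mouse cursor visibility for a hold-to-control-camera input.
; Pressing the ToControlCamera action sets a flag and records the current mouse position, and releasing it clears the flag.
; Each Tick hides the cursor while the flag is set and warps it back to the recorded position, so it reappears where it was pressed.
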(event `self.ReceiveBeginPlay`
  (`self.Init`))

(event `self.ReceiveTick`
  (params (DeltaSeconds :type "Float (single-precision)"))
  (bind _tocontrolcamera (`self.ToControlCamera`))
  (bind (_recordmouseposition_x _recordmouseposition_y) (`KismetMathLibrary.BreakVector2D` (`self.RecordMousePosition`)))
  (set `self.bShowMouseCursor` (not _tocontrolcamera))
  (if _tocontrolcamera
    (`self.SetMouseLocation` (`KismetMathLibrary.FTrunc` _recordmouseposition_x) (`KismetMathLibrary.FTrunc` _recordmouseposition_y))))

(event `InputAction|ToControlCamera` :consume false
  (params (Key :type "Key Structure"))
  (bind (_locationx _locationy _returnvalue) (`self.GetMousePosition`))
  (:`Pressed`
    (set `self.ToControlCamera` true)
    (if _returnvalue
      (set `self.RecordMousePosition` (`KismetMathLibrary.MakeVector2D` _locationx _locationy))))
  (:`Released`
    (set `self.ToControlCamera` false)))

(fn `Init`
  (set `self.ToControlCamera` false))

(fn `UserConstructionScript`)